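; Game instance Blueprint for StreetBrallers that handles level travel and on-screen messages.
; On Init it creates a persistent messages widget, which is later added to the viewport at a high Z-order and receives displayed text.
; Stage loading opens a level by name and creates a second local player when not online.
; Return-to-menu functions open the main menu, optionally passing a message to the widget.
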(event `self.CreateMessagesWidget`
  (`self.Add Messages Widget`))

(event `self.ReturnToMenu`
  (`self.Return to Menu`))

(event `self.ReturnToMenuWithMessage`
  (params (message :type String))
  (`self.Return to Menu with Message` (`KismetTextLibrary.Conv_StringToText` message)))

(event `self.ReceiveInit`
  (bind _returnvalue (`|CreateWidget` "/Game/Menus/MessagesWidget.MessagesWidget_C"))
  (set `self.Messages Widget` _returnvalue))

(fn `Add Messages Widget`
  (`UserWidget.AddToViewport` (`self.Messages Widget`) 100))

(fn `Display Message`
  (params (`Message Text` :type Text))
  (returns (`Message Widget` :type "/Game/Menus/MessageWidget Object Reference"))
  (bind _message_widget (`/Game/Menus/MessagesWidget.Add Messsage` (`self.Messages Widget`) `Message Text`))
  (return _message_widget))

(fn `Load Stage`
  (params (Stage :type Name))
  (`GameplayStatics.OpenLevel` Stage)
  (if (`/Game/Blueprints/FightBlueprintLibrary.Is Online`)
    _
    (elif (< (`GameplayStatics.GetNumLocalPlayerControllers`) 2)
      (`GameplayStatics.CreatePlayer` -1))))

(fn `Return to Menu`
  (`GameplayStatics.OpenLevel` "Main-menu"))

(fn `Return to Menu with Message`
  (params (`Message Text` :type Text))
  (`GameplayStatics.OpenLevel` "Main-menu")
  (`self.Display Message` `Message Text`))