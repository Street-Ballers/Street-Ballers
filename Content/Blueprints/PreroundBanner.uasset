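; PreroundBanner is an actor that appears during the pre-round phase and hides when the round begins.
; On BeginPlay it finds the Logic actor and binds to its OnPreRound and OnBeginRound dispatchers to toggle its in-game visibility.
; A timer event that would call BeginRound on Logic remains in the graph, but the node that sets that timer is disconnected and never runs.
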(event `self.ReceiveBeginPlay`
  (bind _returnvalue (`GameplayStatics.GetActorOfClass` "/Script/menu.Logic"))
  (set `self.logic_instance` _returnvalue)
  (add `Logic.OnPreRound` (`self.logic_instance`) (delegate `OnPreRound Event`))
  (add `Logic.OnBeginRound` (`self.logic_instance`) (delegate `OnBeginRoun Event`)))

(event `OnPreRound Event`
  (`self.SetActorHiddenInGame` false))

(event `OnBeginRoun Event`
  (`self.SetActorHiddenInGame` true))

(event `OnPreRoundTimer_Event`
  (`Logic.beginRound` (`self.logic_instance`)))

(fn `UserConstructionScript`)