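; Player 2's animation Blueprint, which shows that fighter's current action as a 2D flipbook.
; BeginPlay finds and caches the Logic actor.
; Each Tick queries Logic for player index 1's animation state and switches the render component's flipbook to match: idle, walking, damaged, block or strong high punch.
; Character selection is unfinished, with a noted need for an enum and an unconnected flipbook assignment.
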(event `self.ReceiveTick`
  (params (DeltaSeconds :type "Float (single-precision)"))
  ;[1 1 1] Tick Function
  (`self.UpdateAnimation`))

(event `self.ReceiveBeginPlay`
  ;[1 1 1] Setup for Character
  (bind _returnvalue (`GameplayStatics.GetActorOfClass` "/Script/menu.Logic"))
  (set `self.logic_instance` _returnvalue)
  ;;[1 1 1] Set character to use ... need enum for selected char
  (switch `/Engine/EditorResources/FieldNodes/_Resources/Enum_Field` "NewEnumerator0"))

(event `UpdateAnimation`
  ;[1 1 1] Animation Updater...need switch for actions/enum
  (bind _returnvalue (`Logic.playerAnimation` (`self.logic_instance`) 1))
  (switch `EAnimation` _returnvalue
    (:`Idle`
      ;;[1 1 1] Idle/Walk
      (`PaperFlipbookComponent.SetFlipbook` (`self.RenderComponent`) (`self.idle`)))
    (:`WalkBackward`
      (`PaperFlipbookComponent.SetFlipbook` (`self.RenderComponent`) (`self.bw`)))
    (:`WalkForward`
      ;;[1 1 1] Walk Foward
      (`PaperFlipbookComponent.SetFlipbook` (`self.RenderComponent`) (`self.fw`)))
    (:`Damaged`
      (`PaperFlipbookComponent.SetFlipbook` (`self.RenderComponent`) (`self.damaged`)))
    (:`Block`
      ;;[1 1 1] Block
      (`PaperFlipbookComponent.SetFlipbook` (`self.RenderComponent`) (`self.block`)))
    (:`StHP`
      ;;[1 1 1] Strong High Punch
      (`PaperFlipbookComponent.SetFlipbook` (`self.RenderComponent`) (`self.hp`)))))

(fn `UserConstructionScript`)