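; Utility actor Blueprint that uniformly rescales a whole level through the RescaleLevel_Event custom event.
; The event gathers every Actor in the world and multiplies each one's 3D scale and world location by ScaleMultiplier, scaling the layout about the world origin.
; It applies no class filter and moves actors without sweeping; BeginPlay, Tick, overlap and the construction script do nothing.
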(event `Rescale Level_Event`
  (bind _outactors (`GameplayStatics.GetAllActorsOfClass` "/Script/Engine.Actor"))
  (bind _output_get (set `self.all actors` _outactors))
  (for _array_element _output_get
    (`self.SetActorScale3D` _array_element (* (`self.GetActorScale3D` _array_element) (`self.scale multiplier`)))
    (`self.K2_SetActorLocation` _array_element (* (`self.K2_GetActorLocation` _array_element) (`self.scale multiplier`)) false false)))

(fn `UserConstructionScript`)