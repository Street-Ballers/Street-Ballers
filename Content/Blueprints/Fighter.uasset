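; Fighter is the visual actor for one player, mirroring state held by a separate Logic actor as a Paper2D flipbook.
; It finds the Logic actor on BeginPlay, then each tick queries it by PlayerNumber for animation, frame, position and facing.
; The animation indexes a Flipbooks collection, the playback frame is set directly with events firing, and facing flips the actor's yaw.
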(event `self.ReceiveTick`
  (params (DeltaSeconds :type "Float (single-precision)"))
  ;[1 1 1] Tick Function
  (`self.UpdateAnimation`)
  (`self.FrameSet`)
  (bind _returnvalue (`Logic.playerPos` (`self.logic_instance`) (`self.playerNumber`)))
  (bind _returnvalue_2 (`Logic.playerIsFacingRight` (`self.logic_instance`) (`self.playerNumber`)))
  (`self.K2_SetActorLocationAndRotation` _returnvalue (`KismetMathLibrary.MakeRotator` 0.0 0.0 (`KismetMathLibrary.SelectFloat` 90.0 -90.0 _returnvalue_2))))

(event `self.ReceiveBeginPlay`
  ;[1 1 1] Setup for Character
  ;;[1 1 1] Get Logic
  (bind _returnvalue (`GameplayStatics.GetActorOfClass` "/Script/menu.Logic"))
  (set `self.logic_instance` _returnvalue))

(event `UpdateAnimation`
  ;[1 1 1] Animation Updater...need switch for actions/enum
  (bind _returnvalue (`Logic.playerAnimation` (`self.logic_instance`) (`self.playerNumber`)))
  (`PaperFlipbookComponent.SetFlipbook` (`self.PaperFlipbook`) (`|GetArrayItem` (`self.flipbooks`) _returnvalue)))

(event `FrameSet`
  ;[1 1 1] Sets the frame of the sprite
  (bind _returnvalue (`Logic.playerFrame` (`self.logic_instance`) (`self.playerNumber`)))
  (`PaperFlipbookComponent.SetPlaybackPositionInFrames` (`self.PaperFlipbook`) _returnvalue true))

(fn `UserConstructionScript`)