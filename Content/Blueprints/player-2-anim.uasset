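; Player 2's Paper2D flipbook animation driver for a fighting game, mirroring state held by a Logic actor found at BeginPlay.
; Each tick it reads the animation enum for player index 1 and swaps the idle, walk, damaged, block or high-punch flipbook only when the move changes.
; For every listed state except Idle, it also sets the flipbook's playback frame from Logic, so the logic drives animation timing.
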(event `self.ReceiveTick`
  (params (DeltaSeconds :type "Float (single-precision)"))
  ;[1 1 1] Tick Function
  (`self.UpdateAnimation`)
  (`self.FrameSet`))

(event `self.ReceiveBeginPlay`
  ;[1 1 1] Setup for Character
  ;;[1 1 1] Get Logic
  (bind _returnvalue (`GameplayStatics.GetActorOfClass` "/Script/menu.Logic"))
  (set `self.logic_instance` _returnvalue))

(event `UpdateAnimation`
  ;[1 1 1] Animation Updater...need switch for actions/enum
  (bind _returnvalue (`Logic.playerAnimation` (`self.logic_instance`) 1))
  (switch `EAnimation` _returnvalue
    (:`Idle`
      (bind _output_get (set `self.currmove` 0))
      (if (!= _output_get (`self.previousmove`))
        (switch `EAnimation` _returnvalue :!label _label
          (:`Idle`
            ;;[1 1 1] Idle
            (`PaperFlipbookComponent.SetFlipbook` (`self.RenderComponent`) (`self.idle`))
            (set `self.previousmove` 0))
          (:`WalkBackward`
            ;;[1 1 1] Walk Backwards
            (`PaperFlipbookComponent.SetFlipbook` (`self.RenderComponent`) (`self.bw`))
            (set `self.previousmove` 1))
          (:`WalkForward`
            ;;[1 1 1] Walk Foward
            (`PaperFlipbookComponent.SetFlipbook` (`self.RenderComponent`) (`self.fw`))
            (set `self.previousmove` 2))
          (:`Damaged`
            ;;[1 1 1] Damaged
            (`PaperFlipbookComponent.SetFlipbook` (`self.RenderComponent`) (`self.damaged`))
            (set `self.previousmove` 3))
          (:`Block`
            ;;[1 1 1] Block
            (`PaperFlipbookComponent.SetFlipbook` (`self.RenderComponent`) (`self.block`))
            (set `self.previousmove` 4))
          (:`StHP`
            ;;[1 1 1] Strong High Punch
            (`PaperFlipbookComponent.SetFlipbook` (`self.RenderComponent`) (`self.hp`))
            (set `self.previousmove` 5)))))
    (:`WalkBackward`
      (bind _output_get_2 (set `self.currmove` 1))
      (if (!= _output_get_2 (`self.previousmove`))
        (goto _label)))
    (:`WalkForward`
      (bind _output_get_3 (set `self.currmove` 2))
      (if (!= _output_get_3 (`self.previousmove`))
        (goto _label)))
    (:`Damaged`
      (bind _output_get_4 (set `self.currmove` 3))
      (if (!= _output_get_4 (`self.previousmove`))
        (goto _label)))
    (:`Block`
      (bind _output_get_5 (set `self.currmove` 4))
      (if (!= _output_get_5 (`self.previousmove`))
        (goto _label)))
    (:`StHP`
      (bind _output_get_6 (set `self.currmove` 5))
      (if (!= _output_get_6 (`self.previousmove`))
        (goto _label)))))

(event `FrameSet`
  (bind _logic_instance (`self.logic_instance`))
  ;[1 1 1] Frame Set
  (bind _returnvalue (`Logic.playerAnimation` _logic_instance 1))
  (switch `EAnimation` _returnvalue
    (:`WalkBackward`
      _)
    (:`WalkForward`
      _)
    (:`Damaged`
      _)
    (:`Block`
      _)
    (:`StHP`
      _))
  (bind _returnvalue_2 (`Logic.playerFrame` _logic_instance 1))
  (`PaperFlipbookComponent.SetPlaybackPositionInFrames` (`self.RenderComponent`) _returnvalue_2 true))

(fn `UserConstructionScript`)