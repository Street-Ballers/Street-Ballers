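; Blueprint function library of shared helpers for the Street Brallers fighting game.
; It reports online or offline state from the standalone check and reads the local player number from the first LogicPlayerController.
; It also exposes the StreetBrallersGameInstanceB cast and forwards display messages to that game instance.
; For local play, it creates a second player controller when fewer than two local ones exist.
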(fn `Create Second PlayerController`
  (bind _street_brallers_game_instance_b (`self.Get StreetBrallersGameInstanceB` (`local.__WorldContext`)))
  (if (`self.Is Online` _street_brallers_game_instance_b)
    _
    (elif (< (`GameplayStatics.GetNumLocalPlayerControllers` null) 2)
      (`GameplayStatics.CreatePlayer` null))))

(fn `Display Message`
  (params (`Message Text` :type Text))
  (returns (`Message Widget` :type "/Game/Menus/MessageWidget Object Reference"))
  (bind _street_brallers_game_instance_b (`self.Get StreetBrallersGameInstanceB` (`local.__WorldContext`)))
  (bind _message_widget (`/Game/Blueprints/StreetBrallersGameInstanceB.Display Message` _street_brallers_game_instance_b `Message Text`))
  (return _message_widget))

(fn `Get Local Player Number`
  (returns (`Player Number` :type Integer))
  (bind _aslogic_player_controller (cast `LogicPlayerController` (`GameplayStatics.GetPlayerController` (`local.__WorldContext`))))
  (bind _returnvalue (`LogicPlayerController.getPlayerNumber` _aslogic_player_controller))
  (return _returnvalue))

(fn `Get StreetBrallersGameInstanceB`
  (returns (`Street Brallers Game Instance B` :type "/Game/Blueprints/StreetBrallersGameInstanceB Object Reference"))
  (bind _asstreet_brallers_game_instance_b (cast `/Game/Blueprints/StreetBrallersGameInstanceB` (`GameplayStatics.GetGameInstance` null)))
  (return _asstreet_brallers_game_instance_b))

(fn `Is Offline`
  (returns (IsOffline :type Boolean))
  (return (`KismetSystemLibrary.IsStandalone` (`local.__WorldContext`))))

(fn `Is Online`
  (returns (`Is Online` :type Boolean))
  (return (not (`self.Is Offline` (`local.__WorldContext`)))))